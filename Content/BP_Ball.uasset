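; BP_Ball is a ball actor that moves in a straight line and bounces off surfaces it hits.
; Each Tick it sweeps along Direction at Speed, then reflects Direction about the sweep's hit normal, with the branch condition fixed to true rather than a hit check.
; Overlapping a KillZVolume fires the OnDeat dispatcher and destroys the ball.
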(event `self.ReceiveActorBeginOverlap`
  (params (OtherActor :type "Actor Object Reference"))
  (cast `KillZVolume` OtherActor)
  (`self.OnDeat`)
  (`self.K2_DestroyActor`))

(event `self.ReceiveTick`
  (params (DeltaSeconds :type "Float (single-precision)"))
  (bind _sweephitresult (`self.K2_AddActorWorldOffset` (* (* (`self.Direction`) (`self.Speed`)) DeltaSeconds) true))
  (if true
    (set `self.Direction` (`KismetMathLibrary.GetReflectionVector` (`self.Direction`) (`.Normal` (`GameplayStatics.BreakHitResult` _sweephitresult))))))

(fn `UserConstructionScript`)