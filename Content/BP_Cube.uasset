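; BP_Cube is a breakable block that takes damage when hit by a BP_Ball and is destroyed when its Live count runs out.
; The construction script randomly gives each cube one or two lives and picks a matching material.
; Each ball hit calls Ballishit, which decrements Live, switches to the grime material at one life left, and destroys the actor at zero or below.
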(event `self.ReceiveHit`
  (params (MyComp :type "PrimitiveComponent Object Reference") (Other :type "Actor Object Reference") (OtherComp :type "PrimitiveComponent Object Reference") (bSelfMoved :type Boolean) (HitLocation :type "Vector Structure") (HitNormal :type "Vector Structure") (NormalImpulse :type "Vector Structure") (Hit :type "HitResult Structure (by ref)"))
  (cast `/Game/BP_Ball` Other)
  (`self.Ballishit`))

(event `Ballishit`
  (bind _result (`/Engine/EditorBlueprintResources/StandardMacros.DecrementInt` (`self.live`))
    (:`  `
      (if (== _result 1)
        (`PrimitiveComponent.SetMaterial` (`self.Cube`) 0 "/Game/StarterContent/Materials/M_Concrete_Grime.M_Concrete_Grime")
        (elif (<= _result 0)
          (`self.K2_DestroyActor`))))))

(fn `UserConstructionScript`
  (bind _cube (`self.Cube`))
  (bind _output_get (set `self.live` (`KismetMathLibrary.RandomIntegerInRange` 1 2)))
  (switch `int` _output_get
    (:`1`
      (`PrimitiveComponent.SetMaterial` _cube 0 "/Game/StarterContent/Materials/M_Concrete_Grime.M_Concrete_Grime"))
    (:`2`
      (`PrimitiveComponent.SetMaterial` _cube 0 "/Game/StarterContent/Materials/M_CobbleStone_Smooth.M_CobbleStone_Smooth"))))